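; BP_Crystal is a collectible crystal actor that the player picks up by overlapping it.
; An IsPlayer check against player pawn 0 gates the overlap, then caches the crystal's location, scale and point light intensity.
; A timeline lerps the crystal toward the player's current position while shrinking it to zero and fading its light, then destroys the actor.
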(event EventBeginPlay)

(event Collision|EventActorBeginOverlap
  (params (OtherActor :type Actor%20Object%20Reference))
  (Utilities|IsPlayer OtherActor
    (:IsPlayer
      (Variables|Default|SetLerp%20Start%20Location (Transformation|GetActorLocation))
      (Variables|Default|SetStart%20Scale (Transformation|GetActorScale3D))
      (Variables|Default|SetStart%20Light%20Intensity (Variables|/Script/Engine.LightComponentBase|GetIntensity (Variables|Default|GetCrystal%20Point%20Light)))
      (bind (_direction _collection_progress _scale_progress _time_intensity) (Timeline|Collection%20Timeline Play)
        (:Update
          (Transformation|SetActorLocation (Math|Vector|Lerp(Vector) (Variables|Default|GetLerp%20Start%20Location) (Transformation|GetActorLocation (Game|Player|GetPlayerPawn 0)) _collection_progress) false false)
          (Transformation|SetActorScale3D (Math|Vector|Lerp(Vector) (Variables|Default|GetStart%20Scale) "0, 0, 0" _scale_progress))
          (Rendering|Components|Light|SetIntensity (Variables|Default|GetCrystal%20Point%20Light) (Math|Float|Lerp (Variables|Default|GetStart%20Light%20Intensity) 0.0 _time_intensity)))
        (:Finished
          (Actor|DestroyActor))))))

(event EventTick
  (params (DeltaSeconds :type Float%20%28single-precision%29)))

(fn ConstructionScript)