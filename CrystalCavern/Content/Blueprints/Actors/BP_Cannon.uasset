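; BP_Cannon is a cannon actor that automatically fires projectiles on a repeating cycle from BeginPlay.
; After a fire-rate delay, it spawns a BP_Projectile at the spawn point's location and rotation, using a configurable scale.
; A timeline then animates the barrel along its relative Y axis.
; The timeline's Cannon Fired event track restarts the delay, forming the firing loop without Tick.
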(event EventBeginPlay
  (Utilities|FlowControl|Delay (Variables|CannonProperties|GetCannon%20Fire%20Rate) :!label _label)
  (CallFunction|SpawnProyectile)
  (bind _cannon_barrel_location (Timeline|Cannon%20Fire%20Timeline PlayFromStart)
    (:Update
      (CallFunction|MoveCannonBarrel _cannon_barrel_location))
    (:Cannon%20Fired
      (goto _label))))

(event Collision|EventActorBeginOverlap
  (params (OtherActor :type Actor%20Object%20Reference)))

(event EventTick
  (params (DeltaSeconds :type Float%20%28single-precision%29)))

(fn ConstructionScript)

(fn SpawnProyectile
  (bind _projectile_spawn_point (Variables|Default|GetProjectile%20Spawn%20Point))
  (Game|SpawnActorfromClass "/Game/Blueprints/Actors/BP_Projectile.BP_Projectile_C" (Math|Transform|MakeTransform (Transformation|GetWorldLocation _projectile_spawn_point) (Transformation|GetWorldRotation _projectile_spawn_point) (Math|Conversions|ToVector(Float) (Variables|Default|GetProjectile%20Scale))) "Undefined" 0 0))

(fn MoveCannonBarrel
  (params (Cannon%20Barrel%20Y%20Location :type Float%20%28single-precision%29))
  (Transformation|SetRelativeLocation (Variables|Default|GetCannon%20Barrel) (Math|Vector|MakeVector 0.0 Cannon%20Barrel%20Y%20Location 0.0) false false))